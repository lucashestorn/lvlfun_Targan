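; Player stats component that tracks health, stamina, XP and level for BP_Targan_ThirdPersonCharacter and pushes each change to the character's HUD.
; InitializeCharStats caches the owning character and fills the HUD bars and texts.
; Increase functions clamp current health and stamina to their maximums, while decrease functions return true on depletion.
; Reaching max XP raises the level, resets XP to zero and grows the next threshold with level.
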(event `InitializeCharStats`
  (bind _hud (`/Game/Characters/Targan_Char/BP_Targan_ThirdPersonCharacter.Hud` (`self.PlayerCharBP`)))
  (bind _hud_2 (`/Game/Characters/Targan_Char/BP_Targan_ThirdPersonCharacter.Hud` (`self.PlayerCharBP`)))
  (bind _hud_3 (`/Game/Characters/Targan_Char/BP_Targan_ThirdPersonCharacter.Hud` (`self.PlayerCharBP`)))
  (bind _asbp_targan_third_person_character (cast `/Game/Characters/Targan_Char/BP_Targan_ThirdPersonCharacter` (`self.GetOwner`)))
  (set `self.PlayerCharBP` _asbp_targan_third_person_character)
  ;[0.151 0.151 0.151] Stamina
  (`ProgressBar.SetPercent` (`/Game/UI/WB_HUD.StaminaBar` _hud) (/ (`self.Current Stamina`) (`self.Max Stamina`)))
  (`TextBlock.SetText` (`/Game/UI/WB_HUD.SPText` _hud) (`KismetTextLibrary.Conv_DoubleToText` (`self.Current Stamina`) "HalfToEven"))
  ;[0.151 0.151 0.151] HP
  (`ProgressBar.SetPercent` (`/Game/UI/WB_HUD.HealthBar` _hud_2) (/ (`self.Current Health`) (`self.Max Health`)))
  (`TextBlock.SetText` (`/Game/UI/WB_HUD.HPText` _hud_2) (`KismetTextLibrary.Conv_DoubleToText` (`self.Current Health`) "HalfToEven"))
  ;[0.151 0.151 0.151] XP
  (`ProgressBar.SetPercent` (`/Game/UI/WB_HUD.XPBar` _hud_3) (/ (`self.XP`) (`self.Max XP`)))
  (`TextBlock.SetText` (`/Game/UI/WB_HUD.XPText` _hud_3) (`|FormatText` "{Current XP} / {Max XP}" (`self.XP`) (`self.Max XP`)))
  ;[0.151 0.151 0.151] Lvl
  (`TextBlock.SetText` (`/Game/UI/WB_HUD.LvlTxt` (`/Game/Characters/Targan_Char/BP_Targan_ThirdPersonCharacter.Hud` (`self.PlayerCharBP`))) (`KismetTextLibrary.Conv_IntToText` (`self.Level`))))

(fn `Decrease Health`
  (params (Damage :type "Float (double-precision)"))
  (returns (`isPlayerDead?` :type Boolean))
  (bind _hud (`/Game/Characters/Targan_Char/BP_Targan_ThirdPersonCharacter.Hud` (`self.PlayerCharBP`)))
  (if (not (<= (`self.Current Health`) 0.0))
    (bind _output_get (set `self.Current Health` (- (`self.Current Health`) Damage)))
    (`ProgressBar.SetPercent` (`/Game/UI/WB_HUD.HealthBar` _hud) (/ _output_get (`self.Max Health`)))
    (`TextBlock.SetText` (`/Game/UI/WB_HUD.HPText` _hud) (`KismetTextLibrary.Conv_DoubleToText` (`self.Current Health`) "HalfToEven"))
    (if (<= (`self.Current Health`) 0.0)
      _
      (else
        (return false))))
  (return true))

(fn `DecreaseStamina`
  (params (`Stamina Dec` :type "Float (double-precision)"))
  (returns (`Not Stamina Left` :type Boolean))
  (bind _hud (`/Game/Characters/Targan_Char/BP_Targan_ThirdPersonCharacter.Hud` (`self.PlayerCharBP`)))
  (if (not (<= (`self.Current Stamina`) 0.0))
    (set `self.Current Stamina` (- (`self.Current Stamina`) `Stamina Dec`))
    (`ProgressBar.SetPercent` (`/Game/UI/WB_HUD.StaminaBar` _hud) (/ (`self.Current Stamina`) (`self.Max Stamina`)))
    (`TextBlock.SetText` (`/Game/UI/WB_HUD.SPText` _hud) (`KismetTextLibrary.Conv_DoubleToText` (`self.Current Stamina`) "HalfToEven"))
    (if (<= (`self.Current Stamina`) 0.0)
      _
      (else
        (return false))))
  (return true))

(fn `Increase Health`
  (params (`Add Health` :type "Float (double-precision)"))
  (bind _hud (`/Game/Characters/Targan_Char/BP_Targan_ThirdPersonCharacter.Hud` (`self.PlayerCharBP`)))
  (set `self.Current Health` (+ (`self.Current Health`) `Add Health`))
  (if (> (`self.Current Health`) (`self.Max Health`))
    (set `self.Current Health` (`self.Max Health`)))
  (`ProgressBar.SetPercent` (`/Game/UI/WB_HUD.HealthBar` _hud) (/ (`self.Current Health`) (`self.Max Health`)))
  (`TextBlock.SetText` (`/Game/UI/WB_HUD.HPText` _hud) (`KismetTextLibrary.Conv_DoubleToText` (`self.Current Health`) "HalfToEven")))

(fn `Increase Lvl`
  (params (`Add Lvl` :type Integer))
  (set `self.Level` (+ (`self.Level`) `Add Lvl`))
  (set `self.Max XP` (+ (`self.Max XP`) (* 100.0 (`self.Level`))))
  (set `self.XP` 0.0)
  (`TextBlock.SetText` (`/Game/UI/WB_HUD.LvlTxt` (`/Game/Characters/Targan_Char/BP_Targan_ThirdPersonCharacter.Hud` (`self.PlayerCharBP`))) (`KismetTextLibrary.Conv_IntToText` (`self.Level`))))

(fn `Increase Max Health`
  (params (`Increase Health` :type "Float (double-precision)"))
  (bind _hud (`/Game/Characters/Targan_Char/BP_Targan_ThirdPersonCharacter.Hud` (`self.PlayerCharBP`)))
  (set `self.Max Health` (+ (`self.Max Health`) `Increase Health`))
  (`ProgressBar.SetPercent` (`/Game/UI/WB_HUD.HealthBar` _hud) (/ (`self.Current Health`) (`self.Max Health`)))
  (`TextBlock.SetText` (`/Game/UI/WB_HUD.HPText` _hud) (`KismetTextLibrary.Conv_DoubleToText` (`self.Current Health`) "HalfToEven")))

(fn `Increase Max Stamina`
  (params (`Add Max Sta` :type "Float (double-precision)"))
  (bind _hud (`/Game/Characters/Targan_Char/BP_Targan_ThirdPersonCharacter.Hud` (`self.PlayerCharBP`)))
  (set `self.Max Stamina` (+ (`self.Max Stamina`) `Add Max Sta`))
  (`ProgressBar.SetPercent` (`/Game/UI/WB_HUD.StaminaBar` _hud) (/ (`self.Current Stamina`) (`self.Max Stamina`)))
  (`TextBlock.SetText` (`/Game/UI/WB_HUD.SPText` _hud) (`KismetTextLibrary.Conv_DoubleToText` (`self.Current Stamina`) "HalfToEven")))

(fn `Increase Stamina`
  (params (`Add Stamina` :type "Float (double-precision)"))
  (bind _hud (`/Game/Characters/Targan_Char/BP_Targan_ThirdPersonCharacter.Hud` (`self.PlayerCharBP`)))
  (set `self.Current Stamina` (+ (`self.Current Stamina`) `Add Stamina`))
  (if (> (`self.Current Stamina`) (`self.Max Stamina`))
    (set `self.Current Stamina` (`self.Max Stamina`)))
  (`ProgressBar.SetPercent` (`/Game/UI/WB_HUD.StaminaBar` _hud) (/ (`self.Current Stamina`) (`self.Max Stamina`)))
  (`TextBlock.SetText` (`/Game/UI/WB_HUD.SPText` _hud) (`KismetTextLibrary.Conv_DoubleToText` (`self.Current Stamina`) "HalfToEven")))

(fn `Increase XP`
  (params (`Add XP` :type "Float (double-precision)"))
  (bind _hud (`/Game/Characters/Targan_Char/BP_Targan_ThirdPersonCharacter.Hud` (`self.PlayerCharBP`)))
  (set `self.XP` (+ (`self.XP`) `Add XP`))
  (`ProgressBar.SetPercent` (`/Game/UI/WB_HUD.XPBar` _hud) (/ (`self.XP`) (`self.Max XP`)))
  (`TextBlock.SetText` (`/Game/UI/WB_HUD.XPText` _hud) (`|FormatText` "{Current XP} / {Max XP}" (`self.XP`) (`self.Max XP`)))
  (if (>= (`self.XP`) (`self.Max XP`))
    (`self.Increase Lvl` 1)))